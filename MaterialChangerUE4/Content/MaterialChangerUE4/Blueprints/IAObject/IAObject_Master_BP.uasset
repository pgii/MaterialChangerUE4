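; IAObject_Master_BP is a base Blueprint for interactable objects in a material changer system.
; Its construction script applies the configured mesh to the StaticMesh component and rebuilds MaterialList from that mesh's materials.
; CheckActiveMaterialSelector looks up a material index in the MaterialSelector map and returns its IsActive flag, or false if absent.
; The Interaction event is an empty stub.
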(event `Interaction`)

(fn `CheckActiveMaterialSelector`
  (params (InteractionMaterialIndex :type Integer))
  (returns (isActive :type Boolean))
  (bind (_value _returnvalue) (`BlueprintMapLibrary.Map_Find` (`self.MaterialSelector`) InteractionMaterialIndex))
  (if _returnvalue
    (return (`.isActive_8_06C0EFD44378D6CD6F5FE1892BEFB5E9` (break `/Game/MaterialChangerUE4/Blueprints/GameStruct/MatetialSelectorStruct` _value)))
    (else
      (return false))))

(fn `UserConstructionScript`
  (bind _staticmesh (`self.StaticMesh`))
  (`KismetArrayLibrary.Array_Clear` (`self.MaterialList`))
  (`StaticMeshComponent.SetStaticMesh` (`self.StaticMesh`) (`self.Mesh`))
  (if (`KismetSystemLibrary.IsValid` (`StaticMeshComponent.StaticMesh` _staticmesh))
    (for _array_element (`MeshComponent.GetMaterials` _staticmesh)
      (`KismetArrayLibrary.Array_Add` (`self.MaterialList`) _array_element))))