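; Controller for the material changer that adds the view-mode HUD and lets the player pick materials on interactive objects.
; Each tick, unless interaction is broken or the player is moving, a short camera trace caches the hit IAObject_Master_BP, its component and material.
; The material slot comes from the hit face index.
; Picker input clears open selector widgets and opens a new one if that slot is active in the object's MaterialSelector map.
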(event `self.ReceiveBeginPlay`
  (bind _returnvalue (`|CreateWidget` "/Game/MaterialChangerUE4/Blueprints/HUD/HUD_VIewMode_BP.HUD_VIewMode_BP_C"))
  (`UserWidget.AddToViewport` _returnvalue 0))

(event `self.ReceiveTick`
  (params (DeltaSeconds :type "Float (single-precision)"))
  (`self.CheckInteractionObject`))

(event `CheckInteractionObject`
  (bind _returnvalue (`GameplayStatics.GetPlayerCameraManager` 0))
  (bind _returnvalue_2 (`self.K2_GetActorLocation` _returnvalue))
  (if (`self.BreakInteraction`)
    (set `self.CurrentInteractionObject` null :!label _label)
    (elif (> (`KismetMathLibrary.VSize` (`self.GetVelocity` (`GameplayStatics.GetPlayerPawn` 0))) 0.0)
      (goto _label)
      (else
        (bind (_outhit _returnvalue_3) (`KismetSystemLibrary.LineTraceSingle` _returnvalue_2 (+ _returnvalue_2 (* (`self.GetActorForwardVector` _returnvalue) 300.0)) "TraceTypeQuery1"))
        (if _returnvalue_3
          (bind (_bblockinghit _binitialoverlap _time _distance _location _impactpoint _normal _impactnormal _physmat _hitactor _hitcomponent _hitbonename _hititem _faceindex) (`GameplayStatics.BreakHitResult` _outhit))
          (bind _asiaobject_master_bp (cast `/Game/MaterialChangerUE4/Blueprints/IAObject/IAObject_Master_BP` _hitactor)
            (:`then`
              (set `self.CurrentInteractionObject` _asiaobject_master_bp)
              (bind (_sectionindex _returnvalue_4) (`PrimitiveComponent.GetMaterialFromCollisionFaceIndex` _hitcomponent _faceindex))
              (set `self.CurrentInteractionMaterialIndex` _sectionindex)
              (set `self.CurrentInteractionMaterial` _returnvalue_4)
              (set `self.ActiveComponent` _hitcomponent))
            (:`CastFailed`
              (set `self.CurrentInteractionObject` null :!label _label_2)
              (set `self.CurrentInteractionMaterialIndex` 0)
              (set `self.CurrentInteractionMaterial` null)))
          (else
            (goto _label_2)))))))

(event `InputAction|Picker`
  (params (Key :type "Key Structure"))
  (:`Pressed`
    (if (`KismetSystemLibrary.IsValid` (`self.CurrentInteractionObject`))
      (`self.Picker`))))

(event `Picker`
  (bind _foundwidgets (`WidgetBlueprintLibrary.GetAllWidgetsOfClass` "/Game/MaterialChangerUE4/Blueprints/HUD/HUD_MaterialSelector_BP.HUD_MaterialSelector_BP_C"))
  (for _array_element _foundwidgets
    (`Widget.RemoveFromParent` _array_element))
  (bind _isactive (`self.CheckActiveMaterialSelector` (`self.CurrentInteractionMaterialIndex`)))
  (if _isactive
    (bind _returnvalue (`|CreateWidget` "/Game/MaterialChangerUE4/Blueprints/HUD/HUD_MaterialSelector_BP.HUD_MaterialSelector_BP_C"))
    (`UserWidget.AddToViewport` _returnvalue 0)
    (bind _asiaobject_master_bp (cast `/Game/MaterialChangerUE4/Blueprints/IAObject/IAObject_Master_BP` (`self.CurrentInteractionObject`)))
    (`/Game/MaterialChangerUE4/Blueprints/HUD/HUD_MaterialSelector_BP.InitSelector` _returnvalue _asiaobject_master_bp (`self.CurrentInteractionMaterialIndex`) (`self.CurrentInteractionMaterial`))))

(fn `CheckActiveMaterialSelector`
  (params (MaterialIndex :type Integer))
  (returns (isActive :type Boolean))
  (bind _asiaobject_master_bp (cast `/Game/MaterialChangerUE4/Blueprints/IAObject/IAObject_Master_BP` (`self.CurrentInteractionObject`))
    (:`then`
      (bind (_value _returnvalue) (`BlueprintMapLibrary.Map_Find` (`/Game/MaterialChangerUE4/Blueprints/IAObject/IAObject_Master_BP.MaterialSelector` _asiaobject_master_bp) MaterialIndex))
      (if _returnvalue
        (return (`.isActive_8_06C0EFD44378D6CD6F5FE1892BEFB5E9` (break `/Game/MaterialChangerUE4/Blueprints/GameStruct/MatetialSelectorStruct` _value)))
        (else
          (return false))))
    (:`CastFailed`
      (return false))))

(fn `UserConstructionScript`)